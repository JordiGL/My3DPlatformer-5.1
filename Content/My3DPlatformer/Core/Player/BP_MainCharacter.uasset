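; Player character for a 3D platformer that tracks collected coins and keys and can enter a celebration state.
; Tick toggles a trail effect whenever the character has velocity.
; Coin pickups update a TextRender counter, while keys accumulate in a gameplay tag container that is debug-printed.
; A CharacterState enum drives the CanMove check, and celebrating switches that state and attaches a Niagara effect to the capsule.
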(event `self.ReceiveBeginPlay`
  (`ActorComponent.Deactivate` (`self.TrailEffect`)))

(event `self.ReceiveTick`
  (params (DeltaSeconds :type "Float (single-precision)"))
  (if (> (`KismetMathLibrary.VSize` (`MovementComponent.Velocity` (`self.CharacterMovement`))) 0.0)
    (`ActorComponent.Activate` (`self.TrailEffect`) false)
    (else
      (`ActorComponent.Deactivate` (`self.TrailEffect`)))))

(fn `AddACoin`
  (bind _output_get (set `self.NumCoins` (+ (`self.NumCoins`) 1)))
  (`TextRenderComponent.K2_SetText` (`self.TextRender`) (`KismetTextLibrary.Conv_IntToText` _output_get false true 2)))

(fn `CanMove`
  (returns (ReturnValue :type Boolean))
  (return (`|EnumEquality` (`self.CharacterState`) "NewEnumerator1")))

(fn `EnterCelebrations`
  (set `self.CharacterState` "NewEnumerator2")
  (`NiagaraFunctionLibrary.SpawnSystemAttached` "/Game/TeachersMarketplace/Assets/VFX/Emitters/Character/NS_Celebrate.NS_Celebrate" (`self.CapsuleComponent`) "None" (0.0 0.0 0.0) (struct) "SnapToTarget"))

(fn `GetAKey`
  (params (KeyToObtain :type "GameplayTag Structure"))
  (bind _keyscollected (`self.KeysCollected`))
  (`BlueprintGameplayTagLibrary.AddGameplayTag` _keyscollected KeyToObtain)
  (`KismetSystemLibrary.PrintString` (`BlueprintGameplayTagLibrary.GetDebugStringFromGameplayTagContainer` _keyscollected)))

(fn `UserConstructionScript`)