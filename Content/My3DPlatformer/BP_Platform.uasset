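; BP_Platform is a moving platform whose path is laid out with a spline.
; The construction script turns each spline point into a relative control point for InterpToMovement and applies the Duration variable to that component.
; The trigger box overlap event is empty; a camera shake and delayed physics drop of the platform mesh remain in the graph but are disconnected.
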(event `self.TriggerBox.OnComponentBeginOverlap`
  (params (OverlappedComponent :type "PrimitiveComponent Object Reference") (OtherActor :type "Actor Object Reference") (OtherComp :type "PrimitiveComponent Object Reference") (OtherBodyIndex :type Integer) (bFromSweep :type Boolean) (SweepResult :type "HitResult Structure (by ref)")))

(fn `UserConstructionScript`
  (`KismetArrayLibrary.Array_Clear` (`self.Control Points`))
  (for _index (range (`SplineComponent.GetNumberOfSplinePoints` (`self.Spline`)))
    (`KismetArrayLibrary.Array_Add` (`self.Control Points`) (make `InterpControlPoint` (`SplineComponent.GetLocationAtSplinePoint` (`self.Spline`) _index "Local"))))
  (set `InterpToMovementComponent.ControlPoints` (`self.Control Points`) (`self.InterpToMovement`))
  (set `InterpToMovementComponent.Duration` (`self.Duration`) (`self.InterpToMovement`)))